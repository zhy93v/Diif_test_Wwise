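; BP_SoundPlayActor_Blue is a test actor that plays a Wwise audio event on repeat while toggled on.
; On BeginPlay it enables input for player 0, and the 9 key flips an IsPlaying flag.
; Turning it on starts a one-second looping timer that posts the Play_Test_Numbering01 Ak event.
; Turning it off clears that timer.
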(event `self.ReceiveBeginPlay`
  (`self.EnableInput` (`GameplayStatics.GetPlayerController` 0)))

(event `Key|Nine`
  (params (Key :type "Key Structure"))
  (:`Pressed`
    (bind _output_get (set `self.IsPlaying` (not (`self.IsPlaying`))))
    (if _output_get
      (bind _returnvalue (`KismetSystemLibrary.K2_SetTimerDelegate` (delegate `PostAkEvent`) 1.0 true))
      (else
        (`KismetSystemLibrary.K2_ClearAndInvalidateTimerHandle` _returnvalue)))))

(event `PostAkEvent`
  (`AkGameObject.PostAkEvent` :`self` (`self.Ak`) :`AkEvent` "/Game/WwiseAudio/Default_Work_Unit/Play_Test_Numbering01.Play_Test_Numbering01"))

(fn `UserConstructionScript`)